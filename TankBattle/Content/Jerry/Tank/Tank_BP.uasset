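; Player-controlled tank Blueprint that handles driving, camera aiming and firing.
; On BeginPlay it passes its barrel and turret components to functions defined outside this graph.
; Axis inputs set left and right track throttles independently and rotate an azimuth gimbal and spring arm for frame-rate-scaled camera aiming.
; The fire action calls Fire, while turret and barrel movement logic lives outside the Blueprint.
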(event `self.ReceiveBeginPlay`
  (`self.setBarrelReference` (`self.Barrel`))
  (`self.setTurretReference` (`self.TankTurret`)))

(event `InputAxis|Left Track Throttle`
  (params (AxisValue :type "Float (single-precision)"))
  ;[1 1 1] Track throttles
  (`TankTrack.setThrottle` (`self.Track Left`) AxisValue))

(event `InputAxis|AimAzimuth`
  (params (AxisValue :type "Float (single-precision)"))
  ;[1 1 1] Aiming the camera arm in X, Y axes
  (`SceneComponent.K2_AddLocalRotation` (`self.Azimuth_Gimbal`) (`KismetMathLibrary.MakeRotator` 0.0 0.0 (* AxisValue (`GameplayStatics.GetWorldDeltaSeconds`) 100.0)) false false))

(event `InputAxis|Right Track Throttle`
  (params (AxisValue :type "Float (single-precision)"))
  ;[1 1 1] Track throttles
  (`TankTrack.setThrottle` (`self.Track Right`) AxisValue))

(event `InputAxis|AimElevation`
  (params (AxisValue :type "Float (single-precision)"))
  ;[1 1 1] Aiming the camera arm in X, Y axes
  (`SceneComponent.K2_AddLocalRotation` (`self.SpringArm`) (`KismetMathLibrary.MakeRotator` 0.0 (* AxisValue (`GameplayStatics.GetWorldDeltaSeconds`) 100.0)) false false))

(event `InputAction|Fire`
  (params (Key :type "Key Structure"))
  ;[1 1 1] Firing projectile
  (:`Pressed`
    (`self.fire`)))

(fn `UserConstructionScript`)